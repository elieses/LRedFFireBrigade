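; BP_Door is an interactable door whose skeletal mesh animation follows the door's state.
; On BeginPlay it caches the door mesh's anim instance, subscribes to the state-change event and pushes the initial state into ABP_Door_Rig_Skeleton's CurrentState.
; Each state change copies the current state to the anim Blueprint again, so animation updates are event-driven, with Tick left unused.
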(event `self.ReceiveBeginPlay`
  (set `self.DoorABP` (`SkeletalMeshComponent.GetAnimInstance` (`self.GetDoorMesh`)))
  (add `self.OnStateChanged` (delegate `OnStateChanged_Event`))
  (bind _asabp_door_rig_skeleton (cast `/Game/CharacterInteraction/Meshes/Door/ABP_Door_Rig_Skeleton` (`self.DoorABP`)))
  (set `/Game/CharacterInteraction/Meshes/Door/ABP_Door_Rig_Skeleton.CurrentState` (`self.GetState`) _asabp_door_rig_skeleton))

(event `OnStateChanged_Event` :!signature `self.OnStateChanged`
  (params (NewState :type "GameplayTag Structure"))
  (bind _asabp_door_rig_skeleton (cast `/Game/CharacterInteraction/Meshes/Door/ABP_Door_Rig_Skeleton` (`self.DoorABP`)))
  (set `/Game/CharacterInteraction/Meshes/Door/ABP_Door_Rig_Skeleton.CurrentState` (`self.GetState`) _asabp_door_rig_skeleton))

(fn `UserConstructionScript`)