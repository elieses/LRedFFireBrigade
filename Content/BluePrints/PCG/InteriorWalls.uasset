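; GenerateInteriorWalls is a custom PCG node that procedurally lays out interior walls on a point grid across multiple floors.
; It drops points lacking a +X neighbour (other neighbour checks are disconnected), then picks a random line.
; Each further segment turns 90 degrees from the previous one, choosing a side by point counts.
; Density encodes empty, wall or one door per segment, and each floor repeats the pass with raised points.
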(fn ExecutewithContext
  (params (InContext :type PCG%20Context%20Structure%20%28by%20ref%29) (Input :type PCG%20Data%20Collection%20Structure%20%28by%20ref%29))
  (bind _returnvalue (Class|PCGDataFunctionLibrary|GetInputs Input))
  (for _array_element _returnvalue
    (LocalVariables|SetTags (.Tags (PCG|TaggedData|BreakTaggedData _array_element)))
    (LocalVariables|SetPins (.Pin (PCG|TaggedData|BreakTaggedData _array_element)))
    (bind _aspcgspatial_data (Utilities|Casting|CastToPCGSpatialData (.Data (PCG|TaggedData|BreakTaggedData _array_element))))
    (bind _output_get (LocalVariables|SetPCG%20Point%20Data (SpatialData|ToPointDatawithContext _aspcgspatial_data InContext)))
    (bind _output_get_2 (LocalVariables|SetPCG%20Points (SpatialData|GetPoints _output_get)))
    (bind _interiorpoints (CallFunction|RemoveBoundaryPoints _output_get_2))
    (bind _output_get_3 (LocalVariables|SetPCG%20Points _interiorpoints))
    (CallFunction|CalculateforThisPoint _output_get_3)
    ;[0.15 0.15 0.15 0.5] 找到一个合适的随机点获取他的Transform
    (Variables|Default|SetRandomSelectedPoint (CallFunction|FindRandomPoint (LocalVariables|GetPCG%20Points)) :!label _label)
    (while (CallFunction|FurthestPointCheck)
      (Variables|Default|SetRandomSelectedPoint (CallFunction|FindRandomPoint (LocalVariables|GetPCG%20Points))))
    (Variables|Default|SetRandomPointTransforms (Utilities|Struct|BreakPCGPoint (Variables|Default|GetRandomSelectedPoint)))
    ;[0.15 0.15 0.15 0.5] 检查墙是否旋转
    (Variables|Default|SetRotatedWall (Utilities|Operators|EqualEqual (.rotation (Variables|Default|GetRandomPointTransforms)) (Math|Rotator|MakeRotator 0.0 0.0 9e+01) 1.0))
    ;[0.15 0.15 0.15 0.5] 将所有点Density设为0
    (for (_array_element_2 _array_index) (LocalVariables|GetPCG%20Points)
      (bind _structout (Utilities|Struct|SetmembersinPCGPoint _array_element_2 0.0))
      (Utilities|Array|SetArrayElem (LocalVariables|GetPCG%20Points) _array_index _structout))
    (bind _index (Utilities|FlowControl|ForLoopwithBreak 1 (Variables|Default|GetWallSegments) :!label _label_2)
      (:LoopBody
        (LocalVariables|SetWallSpawnIndex _index)
        (Utilities|FlowControl|Sequence
          (:then_0
            (if (and (!= (Variables|Default|GetWallSegments) 1) (!= (LocalVariables|GetWallSpawnIndex) 1))
              (Variables|Default|SetRandomSelectedPoint (.OutItem (Utilities|Array|Random (LocalVariables|GetDoorPointList))))
              (while (CallFunction|FurthestPointCheck)
                (bind _output_get_4 (Variables|Default|SetRandomSelectedPoint (.OutItem (Utilities|Array|Random (LocalVariables|GetDoorPointList)))))
                (bind _returnvalue_2 (Utilities|Array|RemoveItem (LocalVariables|GetDoorPointList) _output_get_4))
                (if (not _returnvalue_2)
                  (goto _label_2 Break)))
              (Variables|Default|SetRandomPointTransforms (CallFunction|RotatePoint))
              (Variables|Default|SetRotatedWall (not (Variables|Default|GetRotatedWall)))
              (bind _returnvalue_3 (CallFunction|CalculateDistancetoEdge (LocalVariables|GetPCG%20Points)))
              (Variables|Default|SetWallSide _returnvalue_3)))
          (:then_1
            (Utilities|Array|Clear (LocalVariables|GetDoorPointList))
            (for (_array_element_3 _array_index_2) (LocalVariables|GetPCG%20Points)
              (LocalVariables|SetWallIndex _array_index_2)
              (if (.PlaceWall (CallFunction|ConditionCheck _array_element_3 (LocalVariables|GetWallSpawnIndex)))
                (bind _structout_2 (Utilities|Struct|SetmembersinPCGPoint (.PCGPoint%20Out (CallFunction|ConditionCheck _array_element_3 (LocalVariables|GetWallSpawnIndex))) 1.0))
                (Utilities|Array|SetArrayElem (LocalVariables|GetPCG%20Points) (LocalVariables|GetWallIndex) _structout_2)
                (Utilities|Array|Add (LocalVariables|GetDoorPointList) _structout_2)
                (else
                  (bind _structout_3 (Utilities|Struct|SetmembersinPCGPoint (.PCGPoint%20Out (CallFunction|ConditionCheck _array_element_3 (LocalVariables|GetWallSpawnIndex))) (.Density (CallFunction|ConditionCheck _array_element_3 (LocalVariables|GetWallSpawnIndex)))))
                  (Utilities|Array|SetArrayElem (LocalVariables|GetPCG%20Points) (LocalVariables|GetWallIndex) _structout_3))))
            (Variables|Default|SetRandomSelectedPoint (.OutItem (Utilities|Array|Random (LocalVariables|GetDoorPointList))))
            (bind (_array_element_4 _array_index_3) (Utilities|Array|ForEachLoopwithBreak (LocalVariables|GetPCG%20Points) :!label _label_3)
              (:LoopBody
                (if (and (== (.Transform (Utilities|Struct|BreakPCGPoint _array_element_4)) (.Transform (Utilities|Struct|BreakPCGPoint (Variables|Default|GetRandomSelectedPoint)))) (== (.Density (Utilities|Struct|BreakPCGPoint _array_element_4)) (.Density (Utilities|Struct|BreakPCGPoint (Variables|Default|GetRandomSelectedPoint)))))
                  (bind _structout_4 (Utilities|Struct|SetmembersinPCGPoint _array_element_4 0.6))
                  (Utilities|Array|SetArrayElem (LocalVariables|GetPCG%20Points) _array_index_3 _structout_4)
                  (goto _label_3 Break)))))))
      (:Completed
        (Math|Integer|IncrementInt (LocalVariables|GetFloor%20passes%20completed)
          (:%20%20
            (if (> (Variables|Default|GetFloors) (LocalVariables|GetFloor%20passes%20completed))
              (for (_array_element_5 _array_index_4) (LocalVariables|GetPCG%20Points)
                (Utilities|Array|Add (LocalVariables|GetPCGPointsCollection) _array_element_5)
                (bind _structout_5 (Utilities|Struct|SetmembersinPCGPoint _array_element_5 (Math|Transform|MakeTransform (+ (.location (.Transform (Utilities|Struct|BreakPCGPoint _array_element_5))) (Math|Vector|MakeVector 0.0 0.0 (Variables|Default|GetFloosHeight))) (.rotation (.Transform (Utilities|Struct|BreakPCGPoint _array_element_5))) (.scale (.Transform (Utilities|Struct|BreakPCGPoint _array_element_5))))))
                (Utilities|Array|SetArrayElem (LocalVariables|GetPCG%20Points) _array_index_4 _structout_5))
              (goto _label)
              (else
                (if (== (Variables|Default|GetFloors) 1)
                  _
                  (else
                    (for _array_element_6 (LocalVariables|GetPCGPointsCollection)
                      (Utilities|Array|Add (LocalVariables|GetPCG%20Points) _array_element_6))))
                (SpatialData|SetPoints (LocalVariables|GetPCG%20Point%20Data) (LocalVariables|GetPCG%20Points))
                (Utilities|Array|Add (LocalVariables|GetOutTaggedData) (PCG|TaggedData|MakeTaggedData (LocalVariables|GetPCG%20Point%20Data) (LocalVariables|GetTags) (LocalVariables|GetPins))))))))))
  (return (Utilities|Struct|MakePCGDataCollection (LocalVariables|GetOutTaggedData))))

(fn NodeTitleOverride
  (return "GenerateInteriorWalls"))

(fn CalculateforThisPoint
  (params (PCG%20Points :type Array%20of%20PCG%20Point%20Structures))
  (Variables|Default|SetFuthestPointAlongX 999999.0)
  (Variables|Default|SetFuthestPointAlongY 999999.0)
  (for _array_element PCG%20Points
    (if (< (.x (.location (.Transform (Utilities|Struct|BreakPCGPoint _array_element)))) (Variables|Default|GetFuthestPointAlongX))
      (Variables|Default|SetFuthestPointAlongX (.x (.location (.Transform (Utilities|Struct|BreakPCGPoint _array_element))))))
    (if (< (.y (.location (.Transform (Utilities|Struct|BreakPCGPoint _array_element)))) (Variables|Default|GetFuthestPointAlongY))
      (Variables|Default|SetFuthestPointAlongY (.y (.location (.Transform (Utilities|Struct|BreakPCGPoint _array_element))))))))

(fn FurthestPointCheck
  (bind _randomselectedpoint (Variables|Default|GetRandomSelectedPoint))
  (bind _transform (Utilities|Struct|BreakPCGPoint _randomselectedpoint))
  (return (or (== (.x (.location _transform)) (Variables|Default|GetFuthestPointAlongX)) (== (.y (.location _transform)) (Variables|Default|GetFuthestPointAlongY)))))

(fn ConditionCheck
  (params (PCGPoint :type PCG%20Point%20Structure%20%28by%20ref%29) (WallSpawnIndex :type Integer))
  (bind (_transform _density) (Utilities|Struct|BreakPCGPoint PCGPoint))
  (bind _randompointtransforms (Variables|Default|GetRandomPointTransforms))
  (LocalVariables|SetPCGX (.x (.location _transform)))
  (LocalVariables|SetPCGY (.y (.location _transform)))
  (LocalVariables|SetPCGZ (.z (.location _transform)))
  (LocalVariables|SetPCGRotation (.rotation _transform))
  (LocalVariables|SetPCGDensity _density)
  (LocalVariables|SetRandomPointX (.x (.location _randompointtransforms)))
  (LocalVariables|SetRandomPointY (.y (.location _randompointtransforms)))
  (LocalVariables|SetRandomPointZ (.z (.location _randompointtransforms)))
  (LocalVariables|SetRandomPointRotation (.rotation _randompointtransforms))
  (return (Math|Boolean|ANDBoolean (== (LocalVariables|GetPCGZ) (LocalVariables|GetRandomPointZ)) (Utilities|Operators|EqualEqual (LocalVariables|GetPCGRotation) (LocalVariables|GetRandomPointRotation) 1.0) (select (Variables|Default|GetRotatedWall) (== (LocalVariables|GetPCGX) (LocalVariables|GetRandomPointX)) (== (LocalVariables|GetPCGY) (LocalVariables|GetRandomPointY))) (select (> WallSpawnIndex 1) (select (Variables|Default|GetWallSide) (select (Variables|Default|GetRotatedWall) (> (LocalVariables|GetRandomPointY) (LocalVariables|GetPCGY)) (< (LocalVariables|GetRandomPointX) (LocalVariables|GetPCGX))) (select (Variables|Default|GetRotatedWall) (<= (LocalVariables|GetRandomPointY) (LocalVariables|GetPCGY)) (> (LocalVariables|GetRandomPointX) (LocalVariables|GetPCGX)))) true)) PCGPoint (LocalVariables|GetPCGDensity)))

(fn FindRandomPoint
  (params (InputPin :type Array%20of%20PCG%20Point%20Structures))
  (return (Utilities|Array|Get(acopy) InputPin (Math|Random|RandomInteger (Utilities|Array|Length InputPin)))))

(fn RotatePoint
  (bind _randomselectedpoint (Variables|Default|GetRandomSelectedPoint))
  (bind _transform (Utilities|Struct|BreakPCGPoint _randomselectedpoint))
  (return (Math|Transform|MakeTransform (.location _transform) (Math|Rotator|MakeRotator (.roll (.rotation _transform)) (.pitch (.rotation _transform)) (Math|Float|SelectFloat 0.0 9e+01 (Variables|Default|GetRotatedWall))) (.scale _transform))))

(fn CalculateDistancetoEdge
  (params (PCGPoints :type Array%20of%20PCG%20Point%20Structures))
  (bind _randompointtransforms (Variables|Default|GetRandomPointTransforms))
  (for _array_element PCGPoints
    (LocalVariables|SetPCGX (.x (.location (.Transform (Utilities|Struct|BreakPCGPoint _array_element)))))
    (LocalVariables|SetPCGY (.y (.location (.Transform (Utilities|Struct|BreakPCGPoint _array_element)))))
    (LocalVariables|SetPCGZ (.z (.location (.Transform (Utilities|Struct|BreakPCGPoint _array_element)))))
    (LocalVariables|SetPCGRotation (.rotation (.Transform (Utilities|Struct|BreakPCGPoint _array_element))))
    (LocalVariables|SetPCGDensity (.Density (Utilities|Struct|BreakPCGPoint _array_element)))
    (LocalVariables|SetRandomPointX (.x (.location _randompointtransforms)))
    (LocalVariables|SetRandomPointY (.y (.location _randompointtransforms)))
    (LocalVariables|SetRandomPointZ (.z (.location _randompointtransforms)))
    (LocalVariables|SetRandomPointRotation (.rotation _randompointtransforms))
    (if (and (Utilities|Operators|EqualEqual (LocalVariables|GetRandomPointRotation) (LocalVariables|GetPCGRotation) 1.0) (== (select (Variables|Default|GetRotatedWall) (LocalVariables|GetRandomPointY) (LocalVariables|GetRandomPointX)) (select (Variables|Default|GetRotatedWall) (LocalVariables|GetPCGY) (LocalVariables|GetPCGX))))
      (Math|Float|CompareFloat (select (Variables|Default|GetRotatedWall) (LocalVariables|GetRandomPointX) (LocalVariables|GetRandomPointY)) (select (Variables|Default|GetRotatedWall) (LocalVariables|GetPCGX) (LocalVariables|GetPCGY))
        (:>
          (Math|Integer|IncrementInt (LocalVariables|GetWallSideA)))
        (:<
          (Math|Integer|IncrementInt (LocalVariables|GetWallSideB))))))
  (return (> (LocalVariables|GetWallSideB) (LocalVariables|GetWallSideA))))

(fn HasNeighbor
  (params (Points :type Array%20of%20PCG%20Point%20Structures) (TargetX :type Float%20%28double-precision%29) (TargetY :type Float%20%28double-precision%29) (TargetZ :type Float%20%28double-precision%29))
  (for _array_element Points
    (if (Math|Boolean|ANDBoolean (< (Math|Float|Absolute(Float) (- (.x (.location (.Transform (Utilities|Struct|BreakPCGPoint _array_element)))) TargetX)) 1.0) (< (Math|Float|Absolute(Float) (- (.y (.location (.Transform (Utilities|Struct|BreakPCGPoint _array_element)))) TargetY)) 1.0) (== (.z (.location (.Transform (Utilities|Struct|BreakPCGPoint _array_element)))) TargetZ))
      (return (Math|Boolean|ANDBoolean (< (Math|Float|Absolute(Float) (- (.x (.location (.Transform (Utilities|Struct|BreakPCGPoint _array_element)))) TargetX)) 1.0) (< (Math|Float|Absolute(Float) (- (.y (.location (.Transform (Utilities|Struct|BreakPCGPoint _array_element)))) TargetY)) 1.0) (== (.z (.location (.Transform (Utilities|Struct|BreakPCGPoint _array_element)))) TargetZ)))))
  (return false))

(fn RemoveBoundaryPoints
  (params (PCG%20Points :type Array%20of%20PCG%20Point%20Structures))
  (for _array_element PCG%20Points
    (bind _output_get (LocalVariables|SetTargetPoint _array_element))
    (LocalVariables|SetX (.x (.location (.Transform (Utilities|Struct|BreakPCGPoint _output_get)))))
    (LocalVariables|SetY (.y (.location (.Transform (Utilities|Struct|BreakPCGPoint _output_get)))))
    (LocalVariables|SetZ (.z (.location (.Transform (Utilities|Struct|BreakPCGPoint _output_get)))))
    (Utilities|FlowControl|Sequence
      (:then_0
        (bind _returnvalue (CallFunction|HasNeighbor PCG%20Points (+ (LocalVariables|GetX) (LocalVariables|GetWallSize)) (LocalVariables|GetY) (LocalVariables|GetZ))))
      (:then_4
        (if _returnvalue
          (Utilities|Array|Add (LocalVariables|GetInteriorPoints) (LocalVariables|GetTargetPoint))))))
  (return (LocalVariables|GetInteriorPoints)))