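; Custom PCG node, SelectRandomPoints, that marks a random set of points in each input by setting their density to DensityToSet.
; It converts spatial data to points, shuffles an index list, picks up to SelectedPointsQuantity indices and overwrites matching points' density.
; All points pass through with their tags and pins, so nothing is removed.
; The index lists and clamped quantity carry over between inputs without being reset.
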(fn ExecutewithContext
  (params (InContext :type PCG%20Context%20Structure%20%28by%20ref%29) (Input :type PCG%20Data%20Collection%20Structure%20%28by%20ref%29))
  (bind _returnvalue (Class|PCGDataFunctionLibrary|GetInputs Input))
  (for _array_element _returnvalue
    (LocalVariables|SetTags (.Tags (PCG|TaggedData|BreakTaggedData _array_element)))
    (LocalVariables|SetPins (.Pin (PCG|TaggedData|BreakTaggedData _array_element)))
    (bind _aspcgspatial_data (Utilities|Casting|CastToPCGSpatialData (.Data (PCG|TaggedData|BreakTaggedData _array_element))))
    (bind _output_get (LocalVariables|SetPCG%20Point%20Data (SpatialData|ToPointDatawithContext _aspcgspatial_data InContext)))
    (bind _output_get_2 (LocalVariables|SetPCG%20Points (SpatialData|GetPoints _output_get)))
    (LocalVariables|SetPoint%20Count (Utilities|Array|Length _output_get_2))
    (LocalVariables|SetSelectMaxPoints (> (Variables|Default|GetSelectedPointsQuantity) (LocalVariables|GetPoint%20Count)))
    (for _index (range 0 (LocalVariables|GetPoint%20Count))
      (Utilities|Array|Add (LocalVariables|GetIndexTracker) _index))
    (Utilities|Array|Shuffle (LocalVariables|GetIndexTracker))
    (if (LocalVariables|GetSelectMaxPoints)
      (Variables|Default|SetSelectedPointsQuantity (+ (LocalVariables|GetPoint%20Count) 1)))
    (for _index_2 (range 1 (Variables|Default|GetSelectedPointsQuantity))
      (Utilities|Array|Add (LocalVariables|GetIndexestoSelect) (Utilities|Array|Get(acopy) (LocalVariables|GetIndexTracker) _index_2)))
    (for (_array_element_2 _array_index) (LocalVariables|GetPCG%20Points)
      (for _array_element_3 (LocalVariables|GetIndexestoSelect)
        (if (== _array_element_3 _array_index)
          (bind _structout (Utilities|Struct|SetmembersinPCGPoint _array_element_2 (Variables|Default|GetDensityToSet)))
          (Utilities|Array|SetArrayElem (LocalVariables|GetPCG%20Points) _array_index _structout))))
    (SpatialData|SetPoints (LocalVariables|GetPCG%20Point%20Data) (LocalVariables|GetPCG%20Points))
    (Utilities|Array|Add (LocalVariables|GetOutTaggedData) (PCG|TaggedData|MakeTaggedData (LocalVariables|GetPCG%20Point%20Data) (LocalVariables|GetTags) (LocalVariables|GetPins))))
  (return (Utilities|Struct|MakePCGDataCollection (LocalVariables|GetOutTaggedData))))

(fn NodeTitleOverride
  (return "SelectRandomPoints"))