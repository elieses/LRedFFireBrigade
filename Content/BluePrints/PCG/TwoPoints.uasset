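; PCG Blueprint node (TowPoints) that marks a random pair of interior points and repeats them across building floors.
; It keeps points with required grid neighbors, then retries random picks until one has a partner 300 units along +Y.
; The pair is distinguished by density, with the rest zeroed.
; For multiple floors, it stacks copies by FloorHeight, adjusting pair density by floor; single-floor runs output nothing.
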(fn ExecutewithContext
  (params (InContext :type PCG%20Context%20Structure%20%28by%20ref%29) (Input :type PCG%20Data%20Collection%20Structure%20%28by%20ref%29))
  (bind _returnvalue (Class|PCGDataFunctionLibrary|GetInputs Input))
  (for _array_element _returnvalue
    (LocalVariables|SetTags (.Tags (PCG|TaggedData|BreakTaggedData _array_element)))
    (LocalVariables|SetPin (.Pin (PCG|TaggedData|BreakTaggedData _array_element)))
    (bind _aspcgspatial_data (Utilities|Casting|CastToPCGSpatialData (.Data (PCG|TaggedData|BreakTaggedData _array_element))))
    (bind _output_get (LocalVariables|SetPCGPointsData (SpatialData|ToPointDatawithContext _aspcgspatial_data InContext)))
    (bind _output_get_2 (Variables|Default|SetPCGPoints (SpatialData|GetPoints _output_get)))
    (bind _interiorpoints (CallFunction|RemoveBoundaryPoints _output_get_2))
    (bind _output_get_3 (Variables|Default|SetPCGPoints _interiorpoints))
    (for (_array_element_2 _array_index) _output_get_3 :!label _label
      (bind _structout (Utilities|Struct|SetmembersinPCGPoint _array_element_2 0.0))
      (Utilities|Array|SetArrayElem (Variables|Default|GetPCGPoints) _array_index _structout))
    (bind _output_get_4 (LocalVariables|SetRandomPointIndex (Math|Random|RandomInteger (Utilities|Array|Length (Variables|Default|GetPCGPoints)))))
    (bind _output_get_5 (Variables|Default|SetRandomSelectPoint (Utilities|Array|Get(acopy) (Variables|Default|GetPCGPoints) (LocalVariables|GetRandomPointIndex))))
    (bind _structout_2 (Utilities|Struct|SetmembersinPCGPoint _output_get_5 1.0))
    (Utilities|Array|SetArrayElem (Variables|Default|GetPCGPoints) _output_get_4 _structout_2)
    (bind (_array_element_3 _array_index_2) (Utilities|Array|ForEachLoopwithBreak (Variables|Default|GetPCGPoints) :!label _label_2)
      (:LoopBody
        (if (== (.Transform (Utilities|Struct|BreakPCGPoint _array_element_3)) (Math|Transform|MakeTransform (Math|Vector|MakeVector (.x (.location (.Transform (Utilities|Struct|BreakPCGPoint (Variables|Default|GetRandomSelectPoint))))) (+ (.y (.location (.Transform (Utilities|Struct|BreakPCGPoint (Variables|Default|GetRandomSelectPoint))))) 3e+02) (.z (.location (.Transform (Utilities|Struct|BreakPCGPoint (Variables|Default|GetRandomSelectPoint)))))) (.rotation (.Transform (Utilities|Struct|BreakPCGPoint (Variables|Default|GetRandomSelectPoint)))) (.scale (.Transform (Utilities|Struct|BreakPCGPoint (Variables|Default|GetRandomSelectPoint))))))
          (bind _structout_3 (Utilities|Struct|SetmembersinPCGPoint _array_element_3 0.9))
          (Utilities|Array|SetArrayElem (Variables|Default|GetPCGPoints) _array_index_2 _structout_3)
          (LocalVariables|SetbFindedPoint (== (.Transform (Utilities|Struct|BreakPCGPoint _array_element_3)) (Math|Transform|MakeTransform (Math|Vector|MakeVector (.x (.location (.Transform (Utilities|Struct|BreakPCGPoint (Variables|Default|GetRandomSelectPoint))))) (+ (.y (.location (.Transform (Utilities|Struct|BreakPCGPoint (Variables|Default|GetRandomSelectPoint))))) 3e+02) (.z (.location (.Transform (Utilities|Struct|BreakPCGPoint (Variables|Default|GetRandomSelectPoint)))))) (.rotation (.Transform (Utilities|Struct|BreakPCGPoint (Variables|Default|GetRandomSelectPoint)))) (.scale (.Transform (Utilities|Struct|BreakPCGPoint (Variables|Default|GetRandomSelectPoint)))))))
          (goto _label_2 Break)))
      (:Completed
        (if (LocalVariables|GetbFindedPoint)
          (if (> (Variables|Default|GetFloors) 1)
            (for (_array_element_4 _array_index_3) (Variables|Default|GetPCGPoints) :!label _label_3
              (bind _structout_4 (Utilities|Struct|SetmembersinPCGPoint _array_element_4 (Math|Float|SelectFloat (Math|Float|SelectFloat (- (.Density (Utilities|Struct|BreakPCGPoint _array_element_4)) 0.2) (.Density (Utilities|Struct|BreakPCGPoint _array_element_4)) (> (.Density (Utilities|Struct|BreakPCGPoint _array_element_4)) 0.5)) (.Density (Utilities|Struct|BreakPCGPoint _array_element_4)) (== (LocalVariables|GetFloors%20Passess%20Completed) 1))))
              (Utilities|Array|Add (LocalVariables|GetPCGPointsCollection) _structout_4)
              (bind _structout_5 (Utilities|Struct|SetmembersinPCGPoint _array_element_4 (Math|Transform|MakeTransform (+ (.location (.Transform (Utilities|Struct|BreakPCGPoint _array_element_4))) (Math|Vector|MakeVector 0.0 0.0 (Variables|Default|GetFloorHeight))) (.rotation (.Transform (Utilities|Struct|BreakPCGPoint _array_element_4))) (.scale (.Transform (Utilities|Struct|BreakPCGPoint _array_element_4)))) (Math|Float|SelectFloat 0.5 (.Density (Utilities|Struct|BreakPCGPoint _array_element_4)) (and (> (.Density (Utilities|Struct|BreakPCGPoint _array_element_4)) 0.5) (== (+ (LocalVariables|GetFloors%20Passess%20Completed) 1) (Variables|Default|GetFloors))))))
              (Utilities|Array|SetArrayElem (Variables|Default|GetPCGPoints) _array_index_3 _structout_5))
            (Math|Integer|IncrementInt (LocalVariables|GetFloors%20Passess%20Completed)
              (:%20%20
                (if (> (Variables|Default|GetFloors) (LocalVariables|GetFloors%20Passess%20Completed))
                  (goto _label_3)
                  (else
                    (for _array_element_5 (LocalVariables|GetPCGPointsCollection)
                      (Utilities|Array|Add (Variables|Default|GetPCGPoints) _array_element_5)
                      (SpatialData|SetPoints (LocalVariables|GetPCGPointsData) (Variables|Default|GetPCGPoints))
                      (Utilities|Array|Add (LocalVariables|GetOutTaggedData) (PCG|TaggedData|MakeTaggedData (LocalVariables|GetPCGPointsData) (LocalVariables|GetTags) (LocalVariables|GetPin)))))))))
          (else
            (goto _label))))))
  (return (Utilities|Struct|MakePCGDataCollection (LocalVariables|GetOutTaggedData))))

(fn NodeTitleOverride
  (return "TowPoints"))

(fn HasNeighbor
  (params (Points :type Array%20of%20PCG%20Point%20Structures) (TargetX :type Float%20%28double-precision%29) (TargetY :type Float%20%28double-precision%29) (TargetZ :type Float%20%28double-precision%29))
  (for _array_element Points
    (if (Math|Boolean|ANDBoolean (< (Math|Float|Absolute(Float) (- (.x (.location (.Transform (Utilities|Struct|BreakPCGPoint _array_element)))) TargetX)) 1.0) (< (Math|Float|Absolute(Float) (- (.y (.location (.Transform (Utilities|Struct|BreakPCGPoint _array_element)))) TargetY)) 1.0) (== (.z (.location (.Transform (Utilities|Struct|BreakPCGPoint _array_element)))) TargetZ))
      (return (Math|Boolean|ANDBoolean (< (Math|Float|Absolute(Float) (- (.x (.location (.Transform (Utilities|Struct|BreakPCGPoint _array_element)))) TargetX)) 1.0) (< (Math|Float|Absolute(Float) (- (.y (.location (.Transform (Utilities|Struct|BreakPCGPoint _array_element)))) TargetY)) 1.0) (== (.z (.location (.Transform (Utilities|Struct|BreakPCGPoint _array_element)))) TargetZ)))))
  (return false))

(fn RemoveBoundaryPoints
  (params (PCG%20Points :type Array%20of%20PCG%20Point%20Structures))
  (for _array_element PCG%20Points
    (bind _output_get (LocalVariables|SetTargetPoint _array_element))
    (LocalVariables|SetX (.x (.location (.Transform (Utilities|Struct|BreakPCGPoint _output_get)))))
    (LocalVariables|SetY (.y (.location (.Transform (Utilities|Struct|BreakPCGPoint _output_get)))))
    (LocalVariables|SetZ (.z (.location (.Transform (Utilities|Struct|BreakPCGPoint _output_get)))))
    (Utilities|FlowControl|Sequence
      (:then_0
        (bind _returnvalue (CallFunction|HasNeighbor PCG%20Points (+ (LocalVariables|GetX) (+ (LocalVariables|GetWallSize) (LocalVariables|GetWallSize))) (LocalVariables|GetY) (LocalVariables|GetZ))))
      (:then_1
        (bind _returnvalue_2 (CallFunction|HasNeighbor PCG%20Points (- (LocalVariables|GetX) (LocalVariables|GetWallSize)) (LocalVariables|GetY) (LocalVariables|GetZ))))
      (:then_2
        (bind _returnvalue_3 (CallFunction|HasNeighbor PCG%20Points (LocalVariables|GetX) (+ (LocalVariables|GetY) (LocalVariables|GetWallSize)) (LocalVariables|GetZ))))
      (:then_3
        (bind _returnvalue_4 (CallFunction|HasNeighbor PCG%20Points (LocalVariables|GetX) (- (LocalVariables|GetY) (LocalVariables|GetWallSize)) (LocalVariables|GetZ))))
      (:then_4
        (if (Math|Boolean|ANDBoolean _returnvalue _returnvalue_2 _returnvalue_3 _returnvalue_4)
          (Utilities|Array|Add (LocalVariables|GetInteriorPoints) (LocalVariables|GetTargetPoint))))))
  (return (LocalVariables|GetInteriorPoints)))